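; Base pickup actor for items collected by overlapping actors that implement PickUpItem_Interface.
; On overlap it ignores other pickups, sends item class, icon and stack size to the other actor via PickUpItemMessage, then destroys itself.
; PushPickUpItemAway applies a velocity-change impulse to the mesh along the player camera's forward vector.
; GetPickUpItemData is a stub returning zero current and maximum stack amounts.
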(event EventBeginPlay)

(event Collision|EventActorBeginOverlap
  (params (OtherActor :type Actor%20Object%20Reference))
  (if (Utilities|DoesObjectImplementInterface OtherActor "/Game/Blueprints/PickUpItem_Interface.PickUpItem_Interface_C")
    (if (not (Utilities|ClassIsChildOf (Utilities|GetClass OtherActor) "BP_PickUpParent_C"))
      (Class|PickUpItemInterface|PickUpItem(Message) OtherActor (Variables|Default|GetItemClass) (Variables|Default|GetItemIcon) (Variables|Default|GetStackSize))
      (Actor|DestroyActor))))

(event EventTick
  (params (DeltaSeconds :type Float%20%28single-precision%29)))

(event EventPushPickUpItemAway
  (bind _returnvalue (Transformation|GetActorLocation))
  (Class|PrimitiveComponent|AddVelocityChangeImpulseatLocation (Variables|Default|GetStaticMesh) (* (Math|Vector|GetForwardVector (Camera|GetCameraRotation (Game|GetPlayerCameraManager 0))) 2.5e+02) (+ _returnvalue (* _returnvalue "15.000000,0.000000,0.000000")) "None"))

(fn ConstructionScript)

(fn GetPickUpItemData
  (return 0 0 0))