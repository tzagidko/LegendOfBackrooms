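; Backroom enemy that chases the player once spotted and punches on contact.
; PawnSensing flags the player as seen and issues an AI MoveTo toward them on each sighting.
; Right after each move request, a collision-sphere overlap check sets the attacking flag and, on overlap, applies damage with a sound and punch montage.
; The attack's DoOnce resets immediately, so sighting events set the attack rate.
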(event OnSeePawn(PawnSensing)
  (params (Pawn :type Pawn%20Object%20Reference))
  (Variables|Default|SetisPlayerSeen true)
  (CallFunction|FollowPlayer))

(event Custom|Follow%20Player
  (if (Variables|Default|GetisPlayerSeen)
    (AI|AIMoveTo self "0, 0, 0" (Game|GetPlayerCharacter 0) 5.0 false
      (:then
        (if (Collision|IsOverlappingActor (Variables|Default|GetCollision%20Sphere) (Game|GetPlayerCharacter 0) :!class /Script/Engine.PrimitiveComponent)
          (Variables|Default|SetisAttacking true)
          (Utilities|FlowControl|DoOnce false :!label _label
            (:Completed
              (Game|Damage|ApplyDamage (Game|GetPlayerCharacter 0) 2e+01 0 0)
              (Audio|PlaySound2D "/Game/Sounds/573377__johnloser__cyber-punch-02.573377__johnloser__cyber-punch-02" 1.0 1.0 0.0 0 0)
              (Animation|PlayAnimMontage "/Game/Anim/AI/PunchMontage.PunchMontage" 1.0 "None")
              (goto _label Reset)))
          (else
            (Variables|Default|SetisAttacking false)))))))

(event EventBeginPlay)

(event Collision|EventActorBeginOverlap
  (params (OtherActor :type Actor%20Object%20Reference)))

(event EventTick
  (params (DeltaSeconds :type Float%20%28single-precision%29)))

(fn ConstructionScript)