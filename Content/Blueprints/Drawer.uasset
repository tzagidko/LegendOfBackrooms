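; Drawer actor that moves the player to preset spots on interaction and exit, apparently as a hide-in or get-in drawer.
; Interract teleports player 0 to the SkeletalMesh transform and snaps DrawerCube001 to DrawerCube002's relative pose.
; GetOut teleports the player to SkeletalMesh1 and snaps the drawer to DrawerCube003's pose.
; Placed components act as pose markers, with no interpolation; the trigger overlap, BeginPlay and Tick events are empty.
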(event OnComponentBeginOverlap(Trigger)
  (params (OverlappedComponent :type Primitive%20Component%20Object%20Reference) (OtherActor :type Actor%20Object%20Reference) (OtherComp :type Primitive%20Component%20Object%20Reference) (OtherBodyIndex :type Integer) (bFromSweep :type Boolean) (SweepResult :type Hit%20Result%20Structure%20%28by%20ref%29)))

(event EventBeginPlay)

(event Collision|EventActorBeginOverlap
  (params (OtherActor :type Actor%20Object%20Reference)))

(event EventTick
  (params (DeltaSeconds :type Float%20%28single-precision%29)))

(event EventInterract
  (bind _skeletalmesh (Variables|Default|GetSkeletalMesh))
  (bind _drawer_cube_002 (Variables|Default|Getdrawer_Cube_002))
  (bind _returnvalue (Transformation|GetWorldTransform _skeletalmesh))
  (Transformation|SetActorTransform (Game|GetPlayerCharacter 0) (Math|Transform|MakeTransform (.location _returnvalue) (.rotation _returnvalue) "1.000000,1.000000,1.000000"))
  (Transformation|SetRelativeLocationAndRotation (Variables|Default|Getdrawer_Cube_001) (Variables|/Script/Engine.SceneComponent|GetRelativeLocation _drawer_cube_002) (Variables|/Script/Engine.SceneComponent|GetRelativeRotation _drawer_cube_002) false false))

(event EventGetOut
  (bind _drawer_cube_003 (Variables|Default|Getdrawer_Cube_003))
  (bind _skeletalmesh1 (Variables|Default|GetSkeletalMesh1))
  (bind _returnvalue (Transformation|GetWorldTransform _skeletalmesh1))
  (Transformation|SetActorTransform (Game|GetPlayerCharacter 0) (Math|Transform|MakeTransform (.location _returnvalue) (.rotation _returnvalue) "1.000000,1.000000,1.000000"))
  (Transformation|SetRelativeLocationAndRotation (Variables|Default|Getdrawer_Cube_001) (Variables|/Script/Engine.SceneComponent|GetRelativeLocation _drawer_cube_003) (Variables|/Script/Engine.SceneComponent|GetRelativeRotation _drawer_cube_003) false false))

(fn ConstructionScript)