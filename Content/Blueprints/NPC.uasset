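; NPC Blueprint that wanders the level and carries a function for adding pickup items to an inventory widget.
; From BeginPlay, FreeRoam moves to a random reachable nearby point and, on success only, repeats after a short delay.
; AddItemToInventory stacks onto a matching entry with room, otherwise creates a W_PickUpItem in the wrap box; nothing here calls it.
; GetPickUpItemData is a stub returning zero counts.
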(event Custom|Free%20Roam
  (AI|AIMoveTo self (.RandomLocation (AI|Navigation|GetRandomReachablePointinRadius (Transformation|GetActorLocation) 2.5e+03 0 0)) 0 5.0 false
    (:OnSuccess
      (Utilities|FlowControl|Delay 2.0)
      (CallFunction|FreeRoam))))

(event EventBeginPlay
  (CallFunction|FreeRoam))

(fn ConstructionScript)

(fn AddItemtoInventory
  (params (ItemClass :type Actor%20Class%20Reference) (ItemIcon :type Texture%202D%20Object%20Reference) (MaxStack :type Integer))
  (if (> MaxStack 1)
    (bind _array_element (Utilities|Array|ForEachLoopwithBreak (Class|PanelWidget|GetAllChildren (Variables|/Game/Blueprints/W_Inventory.W_Inventory_C|GetInventoryBox (Variables|Default|GetInventoryWidget))) :!label _label)
      (:LoopBody
        (bind (_itemclass _currentstackamount _maxstackamount) (Class|PickUpItemInterface|GetPickUpItemData(Message) _array_element))
        (if (== _itemclass ItemClass)
          (if (<= (+ _currentstackamount 1) _maxstackamount)
            (Class|PickUpItemInterface|AddPickUpItemtoStack(Message) _array_element)
            (LocalVariables|SetIsItemAdded? true)
            (goto _label Break))))
      (:Completed
        (if (not (LocalVariables|GetIsItemAdded?))
          (bind _returnvalue (UserInterface|CreateWidget "/Game/Blueprints/W_PickUpItem.W_PickUpItem_C" :!label _label_2))
          (Variables|/Game/Blueprints/W_PickUpItem.W_PickUpItem_C|SetItemClass _returnvalue ItemClass)
          (Class|Image|SetBrush (Variables|/Game/Blueprints/W_PickUpItem.W_PickUpItem_C|GetItemIcon _returnvalue) (Class|WidgetBlueprintLibrary|MakeBrushfromTexture ItemIcon 100 100))
          (Variables|/Game/Blueprints/W_PickUpItem.W_PickUpItem_C|SetMaxStack _returnvalue MaxStack)
          (Class|WrapBox|AddChildtoWrapBox (Variables|/Game/Blueprints/W_Inventory.W_Inventory_C|GetInventoryBox (Variables|Default|GetInventoryWidget)) _returnvalue))))
    (else
      (goto _label_2))))

(fn GetPickUpItemData
  (return 0 0 0))